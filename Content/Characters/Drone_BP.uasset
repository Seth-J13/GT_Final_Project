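; Enemy drone that wanders randomly, chases the player on sight and drops loot when the player touches it.
; Tick issues delayed AI moves to random reachable points until PawnSensing sets IsSeeingPlayer and starts FollowPlayer.
; FollowPlayer's move targets the player controller, and its `then` branch destroys the drone before calling ApplyDamage.
; Box overlap triggers the player's DmgReaction, spawns health or coin pickups around a downward-traced point, then destroys the drone.
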(event `self.ReceiveBeginPlay`)

(event `self.PawnSensing.OnSeePawn`
  (params (Pawn :type "Pawn Object Reference"))
  ; Look for player
  (cast `/Game/ThirdPerson/Blueprints/BP_ThirdPersonCharacter` Pawn)
  (set `self.isSeeingPlayer?` true)
  (`self.Follow Player`))

(event `Follow Player`
  ; Follow Player
  (if (`self.isSeeingPlayer?`)
    (`|AIMoveTo` self (0.0 0.0 0.0) (`GameplayStatics.GetPlayerController` 0)
      (:`then`
        (`self.K2_DestroyActor`)
        (cast `/Game/ThirdPerson/Blueprints/BP_ThirdPersonCharacter` (`GameplayStatics.GetPlayerCharacter` 0))
        (`GameplayStatics.ApplyDamage` null 30.0))
      (:`OnFail`
        (set `self.isSeeingPlayer?` false)))
    (else
      (set `self.isSeeingPlayer?` false))))

(event `self.ReceiveTick`
  (params (DeltaSeconds :type "Float (single-precision)"))
  ; Update where the robot needs to move
  (if (not (`self.isSeeingPlayer?`))
    (`KismetSystemLibrary.Delay` 2.0)
    (`|AIMoveTo` self (`NavigationSystemV1.K2_GetRandomReachablePointInRadius` (`self.K2_GetActorLocation`) 500.0 null null) null 0.0)))

(event `self.Box.OnComponentBeginOverlap`
  (params (OverlappedComponent :type "PrimitiveComponent Object Reference") (OtherActor :type "Actor Object Reference") (OtherComp :type "PrimitiveComponent Object Reference") (OtherBodyIndex :type Integer) (bFromSweep :type Boolean) (SweepResult :type "HitResult Structure (by ref)"))
  ; Kill Robot
  (bind _asbp_third_person_character (cast `/Game/ThirdPerson/Blueprints/BP_ThirdPersonCharacter` OtherActor))
  (`/Game/ThirdPerson/Blueprints/BP_ThirdPersonCharacter.Dmg_Reaction` _asbp_third_person_character)
  (for _ (range (+ (`KismetMathLibrary.RandomInteger` 2) 1))
    (`self.DropLoot`))
  (`self.K2_DestroyActor`))

(event `DropLoot`
  (bind _returnvalue (`self.K2_GetActorLocation`))
  ; Drop Loot when robot is killed
  (bind _outhit (`KismetSystemLibrary.LineTraceSingle` _returnvalue (- _returnvalue (0.0 0.0 250.0)) "TraceTypeQuery1" false (`|MakeArray` (`GameplayStatics.GetPlayerCharacter` 0))))
  (`|SpawnActorFromClass` (select `int` (`KismetMathLibrary.RandomInteger` 10) :`0` "/Game/MyBlueprints/Health_Pickup_BP.Health_Pickup_BP_C" :`1` "/Game/MyBlueprints/Coin_PickUp_BP.Coin_PickUp_BP_C" :!type "Actor Class Reference") (`KismetMathLibrary.MakeTransform` (`NavigationSystemV1.K2_GetRandomReachablePointInRadius` (`.Location` (`GameplayStatics.BreakHitResult` _outhit)) 250.0 null null) (`KismetMathLibrary.MakeRotator` 0.0 0.0 (`KismetMathLibrary.RandomFloatInRange` 0.0))) "Undefined" "MultiplyWithRoot"))

(fn `UserConstructionScript`)