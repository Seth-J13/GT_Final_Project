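; Basic enemy drone that wanders randomly and homes in on the player to deal contact damage, destroying itself.
; PawnSensing spotting the third-person character starts an AIMoveTo chase targeting the player controller; success destroys the drone and applies damage, failure returns it to wandering.
; While no player is seen, Tick uses a Delay to repeatedly move it to random reachable nearby points.
; Box overlap with the player destroys the drone without applying damage.
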(event `self.PawnSensing.OnSeePawn`
  (params (Pawn :type "Pawn Object Reference"))
  (cast `/Game/ThirdPerson/Blueprints/BP_ThirdPersonCharacter` Pawn)
  (set `self.IsSeeingPlayer?` true)
  (`self.FollowPlayer`))

(event `FollowPlayer`
  (if (`self.IsSeeingPlayer?`)
    (`|AIMoveTo` self (0.0 0.0 0.0) (`GameplayStatics.GetPlayerController` 0) 50.0
      (:`OnSuccess`
        (`self.K2_DestroyActor`)
        (bind _asbp_third_person_character (cast `/Game/ThirdPerson/Blueprints/BP_ThirdPersonCharacter` (`GameplayStatics.GetPlayerCharacter` 0)))
        (`GameplayStatics.ApplyDamage` _asbp_third_person_character 30.0))
      (:`OnFail`
        (set `self.IsSeeingPlayer?` false)))
    (else
      (set `self.IsSeeingPlayer?` false))))

(event `self.ReceiveTick`
  (params (DeltaSeconds :type "Float (single-precision)"))
  (bind _randomlocation (`NavigationSystemV1.K2_GetRandomReachablePointInRadius` (`self.K2_GetActorLocation`) 500.0 null null))
  (if (not (`self.IsSeeingPlayer?`))
    (`KismetSystemLibrary.Delay` 2.0)
    (`|AIMoveTo` self (`KismetMathLibrary.MakeVector` (.x _randomlocation) (.y _randomlocation) (.z _randomlocation)) null)))

(event `self.Box.OnComponentBeginOverlap`
  (params (OverlappedComponent :type "PrimitiveComponent Object Reference") (OtherActor :type "Actor Object Reference") (OtherComp :type "PrimitiveComponent Object Reference") (OtherBodyIndex :type Integer) (bFromSweep :type Boolean) (SweepResult :type "HitResult Structure (by ref)"))
  (cast `/Game/ThirdPerson/Blueprints/BP_ThirdPersonCharacter` OtherActor)
  (`self.K2_DestroyActor`))

(fn `UserConstructionScript`)