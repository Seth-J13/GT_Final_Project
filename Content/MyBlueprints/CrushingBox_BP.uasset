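; CrushingBox_BP is a crusher trap whose spikes move along a vertical path and damage the player caught under them.
; After a start delay, the Movement timeline lerps the spikes' relative location, and Crush calls itself again after a pause.
; Box overlap events track whether the third-person character is inside.
; The move is swept, so a blocking hit during overlap applies damage to the player pawn.
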(event `self.Box.OnComponentBeginOverlap`
  (params (OverlappedComponent :type "PrimitiveComponent Object Reference") (OtherActor :type "Actor Object Reference") (OtherComp :type "PrimitiveComponent Object Reference") (OtherBodyIndex :type Integer) (bFromSweep :type Boolean) (SweepResult :type "HitResult Structure (by ref)"))
  ; Kill player if contact
  (cast `/Game/ThirdPerson/Blueprints/BP_ThirdPersonCharacter` OtherActor)
  (set `self.isOverlapping` true))

(event `self.Box.OnComponentEndOverlap`
  (params (OverlappedComponent :type "PrimitiveComponent Object Reference") (OtherActor :type "Actor Object Reference") (OtherComp :type "PrimitiveComponent Object Reference") (OtherBodyIndex :type Integer))
  ; Kill player if contact
  (cast `/Game/ThirdPerson/Blueprints/BP_ThirdPersonCharacter` OtherActor)
  (set `self.isOverlapping` false))

(event `self.ReceiveBeginPlay`
  ; Crusher start & delay
  (`KismetSystemLibrary.Delay` (`self.startDelay`))
  (`self.Crush`))

(event `Crush`
  ; Crush
  (bind (_direction _motion) (`Timeline|Movement`)
    (:`Update`
      (bind _sweephitresult (`SceneComponent.K2_SetRelativeLocation` (`self.Spikes`) (`KismetMathLibrary.VLerp` (0.0 0.0 500.0) (0.0 0.0 0.0) _motion) true false))
      (if (`GameplayStatics.BreakHitResult` _sweephitresult)
        (if (`self.isOverlapping`)
          (bind _asbp_third_person_character (cast `/Game/ThirdPerson/Blueprints/BP_ThirdPersonCharacter` (`GameplayStatics.GetPlayerPawn` 0)))
          (`GameplayStatics.ApplyDamage` _asbp_third_person_character 100.0))))
    (:`Finished`
      (`KismetSystemLibrary.Delay` (`self.Duration`))
      (`self.Crush`))))

(fn `UserConstructionScript`)