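; Puzzle door Blueprint that swings open when enough pressure switches are active and closes when the count drops below the required number.
; SwitchActivated and SwitchDeactivated adjust a running count, compare it to PressureSwitchesNeeded, then play or reverse DoorTimeline.
; The timeline's Alpha drives door yaw up to a quarter turn, and its event track plays the same collapse sound in either direction.
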(event `SwitchActivated`
  (bind _returnvalue (`SceneComponent.K2_GetComponentLocation` (`self.Door`)))
  ; Play door animation based on if a button is being pressed or not
  (`/Engine/EditorBlueprintResources/StandardMacros.IncrementInt` (`self.PressureSwitchesActive`)
    (:`  `
      (if (>= (`self.PressureSwitchesActive`) (`self.PressureSwitchesNeeded`))
        (bind (_direction _alpha) (`Timeline|Door Timeline` :!label _label)
          (:`Update`
            (`SceneComponent.K2_SetRelativeRotation` (`self.Door`) (`KismetMathLibrary.MakeRotator` 0.0 0.0 (* _alpha 90.0)) false false))
          (:`Play Door Sound`
            (switch `ETimelineDirection` _direction
              (:`Forward`
                (`GameplayStatics.PlaySoundAtLocation` "/Game/StarterContent/Audio/Collapse01.Collapse01" _returnvalue (struct) 1.0 1.0 0.0 null null null null))
              (:`Backward`
                (`GameplayStatics.PlaySoundAtLocation` "/Game/StarterContent/Audio/Collapse01.Collapse01" _returnvalue (struct) 1.0 1.0 0.0 null null null null)))))
        (else
          (goto _label :!via `Reverse`))))))

(event `SwitchDeactivated`
  ; Play door animation based on if a button is being pressed or not
  (`/Engine/EditorBlueprintResources/StandardMacros.DecrementInt` (`self.PressureSwitchesActive`)
    (:`  `
      (if (>= (`self.PressureSwitchesActive`) (`self.PressureSwitchesNeeded`))
        (goto _label)
        (else
          (goto _label :!via `Reverse`))))))

(fn `UserConstructionScript`)