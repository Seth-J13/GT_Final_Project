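; AxeHazard_BP is a swinging axe trap that damages the player character on contact.
; After a configurable start delay, the Movement timeline lerps the Scene component's pitch between opposite angles and restarts itself when finished to keep the swing going.
; Overlapping the Box component applies heavy damage to a BP_ThirdPersonCharacter.
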(event `self.ReceiveBeginPlay`
  (`KismetSystemLibrary.Delay` (`self.Delay`))
  (`self.Swing`))

(event `self.Box.OnComponentBeginOverlap`
  (params (OverlappedComponent :type "PrimitiveComponent Object Reference") (OtherActor :type "Actor Object Reference") (OtherComp :type "PrimitiveComponent Object Reference") (OtherBodyIndex :type Integer) (bFromSweep :type Boolean) (SweepResult :type "HitResult Structure (by ref)"))
  (bind _asbp_third_person_character (cast `/Game/ThirdPerson/Blueprints/BP_ThirdPersonCharacter` OtherActor))
  (`GameplayStatics.ApplyDamage` _asbp_third_person_character 100.0))

(event `Swing`
  (bind (_direction _motion) (`Timeline|Movement`)
    (:`Update`
      (`SceneComponent.K2_SetRelativeRotation` (`self.Scene`) (`KismetMathLibrary.RLerp` (struct :`Roll` 80.0) (struct :`Roll` -80.0) _motion true) false false))
    (:`Finished`
      (`self.Swing`))))

(fn `UserConstructionScript`)