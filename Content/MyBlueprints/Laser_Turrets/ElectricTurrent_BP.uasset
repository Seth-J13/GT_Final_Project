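; Electric turret that fires a Niagara beam at the player character while it is inside the NoNoZone trigger.
; Overlap toggles the beam, and Tick calls BeamPlayer to keep its end point on the player.
; A one-second Delay inside that call paces damage, which grows in uneven steps and also sets beam width.
; Leaving the zone switches the beam off and resets the damage.
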(event `self.ReceiveTick`
  (params (DeltaSeconds :type "Float (single-precision)"))
  (if (`self.isSeeingPlayer?`)
    (`self.Beam Player`)))

(event `self.ReceiveBeginPlay`
  ; See player then attack
  (`ActorComponent.Deactivate` (`self.Laser`)))

(event `self.No No Zone.OnComponentBeginOverlap`
  (params (OverlappedComponent :type "PrimitiveComponent Object Reference") (OtherActor :type "Actor Object Reference") (OtherComp :type "PrimitiveComponent Object Reference") (OtherBodyIndex :type Integer) (bFromSweep :type Boolean) (SweepResult :type "HitResult Structure (by ref)"))
  (bind _laser (`self.Laser`))
  ; See player then attack
  (if (== OtherActor (`GameplayStatics.GetPlayerCharacter` 0))
    (set `self.isSeeingPlayer?` true)
    (`ActorComponent.Activate` _laser false)
    (`NiagaraComponent.SetNiagaraVariableFloat` _laser "Beam Width" 2.0)))

(event `self.No No Zone.OnComponentEndOverlap`
  (params (OverlappedComponent :type "PrimitiveComponent Object Reference") (OtherActor :type "Actor Object Reference") (OtherComp :type "PrimitiveComponent Object Reference") (OtherBodyIndex :type Integer))
  ; See player then attack
  (if (== OtherActor (`GameplayStatics.GetPlayerCharacter` 0))
    (set `self.isSeeingPlayer?` false)
    (`ActorComponent.Deactivate` (`self.Laser`))
    (set `self.beamDamage` 0.0)))

(event `Beam Player`
  (bind _beamdamage (`self.beamDamage`))
  (bind (_returnvalue_x _returnvalue_y _returnvalue_z) (`KismetMathLibrary.BreakVector` (`SceneComponent.K2_GetComponentLocation` (`Character.Mesh` (`GameplayStatics.GetPlayerCharacter` 0)))))
  ; Beam Player when in no no zone
  (`NiagaraComponent.SetNiagaraVariableVec3` (`self.Laser`) (`self.Beam Point`) (`KismetMathLibrary.MakeVector` _returnvalue_x _returnvalue_y (+ _returnvalue_z 100.0)))
  (`KismetSystemLibrary.Delay` 1.0)
  (if (<= (`self.beamDamage`) 4.0)
    (set `self.beamDamage` (+ 2.0 (`self.beamDamage`)))
    (elif (<= 28.0 (`self.beamDamage`))
      (set `self.beamDamage` (+ 8.0 (`self.beamDamage`)))
      (else
        (set `self.beamDamage` (+ 10.0 (`self.beamDamage`))))))
  (bind _asbp_third_person_character (cast `/Game/ThirdPerson/Blueprints/BP_ThirdPersonCharacter` (`GameplayStatics.GetPlayerCharacter` 0)))
  (`GameplayStatics.ApplyDamage` _asbp_third_person_character _beamdamage)
  (`NiagaraComponent.SetVariableFloat` (`self.Laser`) "Beam Width" _beamdamage))

(fn `UserConstructionScript`)