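; Puzzle laser switch that disables and enables a list of linked lasers, changing its base material to match.
; PressZone overlaps track proximity, and pressing E while close toggles a pressed flag.
; While close and pressed, Tick alternates between disable and enable each frame through the ChangeMaterial flag.
; The one-second Delay trailing each loop body does not throttle this alternation.
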(event `Key|E`
  (params (Key :type "Key Structure"))
  (:`Pressed`
    (if (`self.isClose?`)
      (set `self.isEPressed?` (not (`self.isEPressed?`))))))

(event `Key|E`
  (params (Key :type "Key Structure"))
  ; Check for interaction with switch
)

(event `self.press zone.OnComponentBeginOverlap`
  (params (OverlappedComponent :type "PrimitiveComponent Object Reference") (OtherActor :type "Actor Object Reference") (OtherComp :type "PrimitiveComponent Object Reference") (OtherBodyIndex :type Integer) (bFromSweep :type Boolean) (SweepResult :type "HitResult Structure (by ref)"))
  ; Check if player is close to switch
  (set `self.isClose?` true))

(event `self.press zone.OnComponentEndOverlap`
  (params (OverlappedComponent :type "PrimitiveComponent Object Reference") (OtherActor :type "Actor Object Reference") (OtherComp :type "PrimitiveComponent Object Reference") (OtherBodyIndex :type Integer))
  ; Check if player is close to switch
  (set `self.isClose?` false))

(event `self.ReceiveTick`
  (params (DeltaSeconds :type "Float (single-precision)"))
  (bind _base (`self.Base`))
  ; Change Material if switched then disable laser
  (if (`self.isClose?`)
    (if (`self.isEPressed?`)
      (if (`self.changeMaterial?`)
        (`PrimitiveComponent.SetMaterial` _base 0 "/Game/PolygonDungeons/Materials/Alternates/M_Dungeon_01_C.M_Dungeon_01_C")
        (set `self.changeMaterial?` false)
        (for _array_element (`self.lasersToStop`)
          (`/Game/MyBlueprints/Laser_Turrets/Puzzle_Turret/pzl_ElectricTurrent_BP.Disable Laser` _array_element)
          (`KismetSystemLibrary.Delay` 1.0 :!label _label))
        (else
          (`PrimitiveComponent.SetMaterial` _base 0 "/Game/PolygonDungeons/Materials/Alternates/M_Dungeon_01_A.M_Dungeon_01_A")
          (set `self.changeMaterial?` true)
          (for _array_element_2 (`self.lasersToStop`)
            (`/Game/MyBlueprints/Laser_Turrets/Puzzle_Turret/pzl_ElectricTurrent_BP.Enable Laser` _array_element_2)
            (goto _label)))))))

(fn `UserConstructionScript`)