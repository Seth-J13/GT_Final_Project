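; Moving platform Blueprint that slides its Cube back and forth along its relative Y axis in an endless loop.
; After BeginPlay and a configurable Delay, PlatformTimeline plays forward, and its OffsetAlpha track scales the offset applied to the Cube.
; When the timeline finishes, its Direction selects the MovePlatformForward or MovePlatformBack event, producing a continuous ping-pong motion.
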(event `self.ReceiveBeginPlay`
  (`|ExecutionSequence`
    (:`then_0`
      (`KismetSystemLibrary.Delay` (`self.Delay`))
      (`self.Move Platform Forward`))
    (:`then_1`
      (bind (_direction _offset_alpha) (`Timeline|Platform Timeline` :`NewTime` 1.0 :!via `SetNewTime` :!label _label)
        (:`Update`
          (`SceneComponent.K2_SetRelativeLocation` (`self.Cube`) (`KismetMathLibrary.MakeVector` 0.0 (* _offset_alpha 300.0)) false false))
        (:`Finished`
          (switch `ETimelineDirection` _direction
            (:`Forward`
              (`self.Move Platform Back`))
            (:`Backward`
              (`self.Move Platform Forward`))))))))

(event `Move Platform Forward`
  (goto _label))

(event `Move Platform Back`
  (goto _label :!via `Reverse`))

(fn `UserConstructionScript`)