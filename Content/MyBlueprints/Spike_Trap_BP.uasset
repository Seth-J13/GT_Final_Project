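; Spike trap Blueprint that moves its spikes and deals heavy damage to the third-person player character.
; TrapActivated waits a configurable delay, then a timeline lerps the Scene component's relative location with sweep, ignoring retriggers until it finishes.
; A blocking sweep hit damages the player only while the character overlaps the Box trigger.
; A separate FailsafeHitbox damages the character on any overlap, independent of trap state.
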(event `self.Box.OnComponentBeginOverlap`
  (params (OverlappedComponent :type "PrimitiveComponent Object Reference") (OtherActor :type "Actor Object Reference") (OtherComp :type "PrimitiveComponent Object Reference") (OtherBodyIndex :type Integer) (bFromSweep :type Boolean) (SweepResult :type "HitResult Structure (by ref)"))
  (cast `/Game/ThirdPerson/Blueprints/BP_ThirdPersonCharacter` OtherActor)
  (set `self.Is overlapping ` true))

(event `self.Box.OnComponentEndOverlap`
  (params (OverlappedComponent :type "PrimitiveComponent Object Reference") (OtherActor :type "Actor Object Reference") (OtherComp :type "PrimitiveComponent Object Reference") (OtherBodyIndex :type Integer))
  (cast `/Game/ThirdPerson/Blueprints/BP_ThirdPersonCharacter` OtherActor)
  (set `self.Is overlapping ` false))

(event `Trap Activated`
  (`KismetSystemLibrary.Delay` (`self.Trap Activation Delay`))
  (if (`self.Is Trap Set?`)
    (set `self.Is Trap Set?` false)
    (bind (_direction _trap_movement) (`Timeline|Trap monevment` :!via `PlayFromStart`)
      (:`Update`
        (bind _sweephitresult (`SceneComponent.K2_SetRelativeLocation` (`self.Scene`) (`KismetMathLibrary.VLerp` (0.0 0.0 0.0) (`self.B`) _trap_movement) true false))
        (if (`GameplayStatics.BreakHitResult` _sweephitresult)
          (if (`self.Is overlapping `)
            (bind _asbp_third_person_character (cast `/Game/ThirdPerson/Blueprints/BP_ThirdPersonCharacter` (`GameplayStatics.GetPlayerPawn` 0)))
            (`GameplayStatics.ApplyDamage` _asbp_third_person_character 100.0))))
      (:`Finished`
        (set `self.Is Trap Set?` true)))))

(event `self.Failsafe hitbox.OnComponentBeginOverlap`
  (params (OverlappedComponent :type "PrimitiveComponent Object Reference") (OtherActor :type "Actor Object Reference") (OtherComp :type "PrimitiveComponent Object Reference") (OtherBodyIndex :type Integer) (bFromSweep :type Boolean) (SweepResult :type "HitResult Structure (by ref)"))
  (bind _asbp_third_person_character (cast `/Game/ThirdPerson/Blueprints/BP_ThirdPersonCharacter` OtherActor))
  (`GameplayStatics.ApplyDamage` _asbp_third_person_character 100.0))

(fn `UserConstructionScript`)