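; A puzzle button actor that opens a linked door when an actor tagged "Heavy" overlaps it.
; The first qualifying overlap sets IsPressed, calls DoorOpened on DoorToOpen and swaps the switch to its "on" material.
; The SwitchActivate timeline then animates the switch's relative Z position.
; Despite the Toggle name, it latches: nothing here resets the flag, reverses the switch or closes the door.
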(event `self.ReceiveActorBeginOverlap`
  (params (OtherActor :type "Actor Object Reference"))
  (if (`self.ActorHasTag` OtherActor "Heavy")
    (if (not (`self.IsPressed?`))
      (set `self.IsPressed?` true)
      ; Make switch move up and down if player is on or off it
      ;; Make door open or close
      (`/Game/MyBlueprints/Secret_Door.Door Opened` (`self.Door to open`))
      (`PrimitiveComponent.SetMaterial` (`self.Switch`) 0 "/Game/MyMaterials/M_Switch_On.M_Switch_On")
      (bind (_direction _switchposition) (`Timeline|SwitchActivate`)
        (:`Update`
          (`SceneComponent.K2_SetRelativeLocation` (`self.Switch`) (`KismetMathLibrary.MakeVector` 0.0 0.0 _switchposition) false false))))))

(fn `UserConstructionScript`)