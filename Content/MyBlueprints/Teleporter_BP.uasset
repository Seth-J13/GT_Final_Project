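; A two-pad teleporter actor that moves the player character between its pads after standing on one for TeleportTime.
; Overlap of either sphere by the player's capsule starts a shared timer that calls Teleport toward the other pad's target location.
; Teleport moves the player and sets OnCoolDown, which gates new timers.
; End overlap waits briefly, rechecks that the player left that sphere, then clears the timer and cooldown.
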(event `self.Sphere.OnComponentBeginOverlap`
  (params (OverlappedComponent :type "PrimitiveComponent Object Reference") (OtherActor :type "Actor Object Reference") (OtherComp :type "PrimitiveComponent Object Reference") (OtherBodyIndex :type Integer) (bFromSweep :type Boolean) (SweepResult :type "HitResult Structure (by ref)"))
  (if (and (not (`self.onCoolDown?`)) (== OtherComp (`Character.CapsuleComponent` (`GameplayStatics.GetPlayerCharacter` 0))))
    (bind _returnvalue (`KismetSystemLibrary.K2_SetTimerDelegate` (delegate `TeleportTo2`) (`self.TeleportTime`)))
    (set `self.TeleportTimer` _returnvalue)))

(event `TeleportTo2`
  (`self.Teleport` (`SceneComponent.K2_GetComponentLocation` (`self.PadTarget2`))))

(event `self.Sphere2.OnComponentBeginOverlap`
  (params (OverlappedComponent :type "PrimitiveComponent Object Reference") (OtherActor :type "Actor Object Reference") (OtherComp :type "PrimitiveComponent Object Reference") (OtherBodyIndex :type Integer) (bFromSweep :type Boolean) (SweepResult :type "HitResult Structure (by ref)"))
  (if (and (not (`self.onCoolDown?`)) (== OtherComp (`Character.CapsuleComponent` (`GameplayStatics.GetPlayerCharacter` 0))))
    (bind _returnvalue (`KismetSystemLibrary.K2_SetTimerDelegate` (delegate `TeleportTo1`) (`self.TeleportTime`)))
    (set `self.TeleportTimer` _returnvalue)))

(event `TeleportTo1`
  (`self.Teleport` (`SceneComponent.K2_GetComponentLocation` (`self.PadTarget1`))))

(event `self.Sphere.OnComponentEndOverlap`
  (params (OverlappedComponent :type "PrimitiveComponent Object Reference") (OtherActor :type "Actor Object Reference") (OtherComp :type "PrimitiveComponent Object Reference") (OtherBodyIndex :type Integer))
  (`KismetSystemLibrary.Delay` 0.1)
  (if (not (`PrimitiveComponent.IsOverlappingActor` (`self.Sphere`) (`GameplayStatics.GetPlayerCharacter` 0)))
    (`KismetSystemLibrary.K2_ClearAndInvalidateTimerHandle` (`self.TeleportTimer`))
    (set `self.onCoolDown?` false)))

(event `self.Sphere2.OnComponentEndOverlap`
  (params (OverlappedComponent :type "PrimitiveComponent Object Reference") (OtherActor :type "Actor Object Reference") (OtherComp :type "PrimitiveComponent Object Reference") (OtherBodyIndex :type Integer))
  (`KismetSystemLibrary.Delay` 0.1)
  (if (not (`PrimitiveComponent.IsOverlappingActor` (`self.Sphere2`) (`GameplayStatics.GetPlayerCharacter` 0)))
    (`KismetSystemLibrary.K2_ClearAndInvalidateTimerHandle` (`self.TeleportTimer`))
    (set `self.onCoolDown?` false)))

(fn `Teleport`
  (params (target :type "Vector Structure"))
  (`self.K2_SetActorLocation` (`GameplayStatics.GetPlayerCharacter` 0) target false false)
  (set `self.onCoolDown?` true))

(fn `UserConstructionScript`)