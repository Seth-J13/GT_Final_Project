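; Puzzle pressure switch that activates a linked door while an actor tagged "Heavy" rests on it.
; The first heavy overlap presses it, notifying DoorToActivate, swapping the switch material, playing a sound at world origin and moving the switch along a timeline.
; On end overlap it rescans remaining actors and releases only when none are heavy, deactivating the door and reversing the timeline.
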(event `self.ReceiveActorBeginOverlap`
  (params (OtherActor :type "Actor Object Reference"))
  (if (`self.ActorHasTag` OtherActor "Heavy")
    (if (not (`self.IsPressed?`))
      (set `self.IsPressed?` true)
      ; Make switch move up and down if player is on or off it
      ;; Make door open or close
      (`/Game/MyBlueprints/pzl_Door_BP.SwitchActivated` (`self.DoorToActivate`))
      (`PrimitiveComponent.SetMaterial` (`self.Switch`) 0 "/Game/MyMaterials/M_Switch_On.M_Switch_On")
      (`GameplayStatics.PlaySoundAtLocation` "/Game/StarterContent/Audio/Collapse01.Collapse01" (0.0 0.0 0.0) (struct) 1.0 1.0 0.0 null null null null)
      (bind (_direction _switchposition) (`Timeline|SwitchActivate` :!label _label)
        (:`Update`
          (`SceneComponent.K2_SetRelativeLocation` (`self.Switch`) (`KismetMathLibrary.MakeVector` 0.0 0.0 _switchposition) false false))))))

(event `self.ReceiveActorEndOverlap`
  (params (OtherActor :type "Actor Object Reference"))
  (set `self.Weighted?` false)
  (for _array_element (`self.GetOverlappingActors` null)
    (if (`self.ActorHasTag` _array_element "Heavy")
      (set `self.Weighted?` true)))
  (if (`self.Weighted?`)
    _
    (elif (not (not (`self.IsPressed?`)))
      (set `self.IsPressed?` false)
      ; Make switch move up and down if player is on or off it
      ;; Make door open or close
      (`/Game/MyBlueprints/pzl_Door_BP.SwitchDeactivated` (`self.DoorToActivate`))
      (`PrimitiveComponent.SetMaterial` (`self.Switch`) 0 "/Game/MyMaterials/M_Switch_Off.M_Switch_Off")
      (`GameplayStatics.PlaySoundAtLocation` "/Game/StarterContent/Audio/Collapse02.Collapse02" (0.0 0.0 0.0) (struct) 1.0 1.0 0.0 null null null null)
      (goto _label :!via `Reverse`))))

(fn `UserConstructionScript`)