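; Rune puzzle elevator that rises when its Top, Middle and Bottom pieces are rotated to the correct yaws.
; Entering the box enables input, with E, F and G each turning one piece 90 degrees, debounced by DoOnce and Delay.
; Overlap also starts a self-rearming timer that prints and checks the yaws, repeatedly triggering an upward root move while they match.
; Leaving disables input and stops that move, but never clears the timer.
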(event `move up`
  (bind _defaultsceneroot (`self.DefaultSceneRoot`))
  (bind (_returnvalue_x _returnvalue_y _returnvalue_z) (`KismetMathLibrary.BreakVector` (`SceneComponent.K2_GetComponentLocation` _defaultsceneroot)))
  (`KismetSystemLibrary.MoveComponentTo` (`self.DefaultSceneRoot`) (`KismetMathLibrary.MakeVector` _returnvalue_x _returnvalue_y (+ _returnvalue_z 100.0)) (`SceneComponent.K2_GetComponentRotation` _defaultsceneroot) :!label _label))

(event `self.Box.OnComponentBeginOverlap`
  (params (OverlappedComponent :type "PrimitiveComponent Object Reference") (OtherActor :type "Actor Object Reference") (OtherComp :type "PrimitiveComponent Object Reference") (OtherBodyIndex :type Integer) (bFromSweep :type Boolean) (SweepResult :type "HitResult Structure (by ref)"))
  ; pay attention to input when in box and tell rotation status
  (`self.EnableInput` (`GameplayStatics.GetPlayerController` 0))
  (`KismetSystemLibrary.PrintString` "E > Rotate Top \nF > Rotate Middle \nG > Rotate Bottom" true true (struct :`R` 1.0 :`G` 0.135668 :`B` 0.847283 :`A` 1.0))
  (`self.get rotation values`))

(event `self.ReceiveBeginPlay`
  ; create reference to player
  (bind _asbp_third_person_character (cast `/Game/ThirdPerson/Blueprints/BP_ThirdPersonCharacter` (`GameplayStatics.GetPlayerCharacter` 0)))
  (set `self.Char Reference` _asbp_third_person_character))

(event `self.Box.OnComponentEndOverlap`
  (params (OverlappedComponent :type "PrimitiveComponent Object Reference") (OtherActor :type "Actor Object Reference") (OtherComp :type "PrimitiveComponent Object Reference") (OtherBodyIndex :type Integer))
  ; pay attention to input when in box and tell rotation status
  (`self.DisableInput` (`GameplayStatics.GetPlayerController` 0))
  (goto _label :!via `Stop`))

(event `get rotation values`
  (bind (_returnvalue_roll _returnvalue_pitch _returnvalue_yaw) (`KismetMathLibrary.BreakRotator` (`SceneComponent.K2_GetComponentRotation` (`self.Bottom`))))
  (bind (_returnvalue_roll_2 _returnvalue_pitch_2 _returnvalue_yaw_2) (`KismetMathLibrary.BreakRotator` (`SceneComponent.K2_GetComponentRotation` (`self.Top`))))
  (bind (_returnvalue_roll_3 _returnvalue_pitch_3 _returnvalue_yaw_3) (`KismetMathLibrary.BreakRotator` (`SceneComponent.K2_GetComponentRotation` (`self.Middle`))))
  ; tell us the rotation and allow something to happen
  (`KismetSystemLibrary.K2_SetTimerDelegate` (delegate `get rotation values`) 0.5)
  (`KismetSystemLibrary.PrintString` (`KismetStringLibrary.Conv_DoubleToString` _returnvalue_yaw_2))
  (`KismetSystemLibrary.PrintString` (`KismetStringLibrary.Conv_DoubleToString` _returnvalue_yaw_3))
  (`KismetSystemLibrary.PrintString` (`KismetStringLibrary.Conv_DoubleToString` _returnvalue_yaw))
  (if (and (`KismetMathLibrary.NearlyEqual_FloatFloat` _returnvalue_yaw_2 (`self.Top Rotation Correct`) 1.0) (`KismetMathLibrary.NearlyEqual_FloatFloat` _returnvalue_yaw_3 (`self.Middle Rotation Correct`) 1.0) (`KismetMathLibrary.NearlyEqual_FloatFloat` _returnvalue_yaw (`self.Bottom Rotation Correct`) 1.0))
    (`KismetSystemLibrary.PrintString` "All Conditions Are Met")
    (`self.move up`)))

(event `Key|E`
  (params (Key :type "Key Structure"))
  (bind _top (`self.Top`))
  (bind (_returnvalue_roll _returnvalue_pitch _returnvalue_yaw) (`KismetMathLibrary.BreakRotator` (`SceneComponent.K2_GetComponentRotation` _top)))
  ; rotate top when e pressed
  (:`Pressed`
    (`/Engine/EditorBlueprintResources/StandardMacros.DoOnce` false :!label _label_2
      (:`Completed`
        (`KismetSystemLibrary.MoveComponentTo` (`self.Top`) (`SceneComponent.RelativeLocation` _top) (`KismetMathLibrary.MakeRotator` 0.0 0.0 (+ _returnvalue_yaw 90.0)))
        (`KismetSystemLibrary.Delay` 0.5)
        (goto _label_2 :!via `Reset`)))))

(event `Key|F`
  (params (Key :type "Key Structure"))
  (bind _middle (`self.Middle`))
  (bind (_returnvalue_roll _returnvalue_pitch _returnvalue_yaw) (`KismetMathLibrary.BreakRotator` (`SceneComponent.K2_GetComponentRotation` _middle)))
  ; rotate middle when f is pressed
  (:`Pressed`
    (`/Engine/EditorBlueprintResources/StandardMacros.DoOnce` false :!label _label_3
      (:`Completed`
        (`KismetSystemLibrary.MoveComponentTo` (`self.Middle`) (`SceneComponent.RelativeLocation` _middle) (`KismetMathLibrary.MakeRotator` 0.0 0.0 (+ _returnvalue_yaw 90.0)))
        (`KismetSystemLibrary.Delay` 0.5)
        (goto _label_3 :!via `Reset`)))))

(event `Key|G`
  (params (Key :type "Key Structure"))
  (bind _bottom (`self.Bottom`))
  (bind (_returnvalue_roll _returnvalue_pitch _returnvalue_yaw) (`KismetMathLibrary.BreakRotator` (`SceneComponent.K2_GetComponentRotation` _bottom)))
  ; bottom rotate
  (:`Pressed`
    (`/Engine/EditorBlueprintResources/StandardMacros.DoOnce` false :!label _label_4
      (:`Completed`
        (`KismetSystemLibrary.MoveComponentTo` (`self.Bottom`) (`SceneComponent.RelativeLocation` _bottom) (`KismetMathLibrary.MakeRotator` 0.0 0.0 (+ _returnvalue_yaw 90.0)))
        (`KismetSystemLibrary.Delay` 0.5)
        (goto _label_4 :!via `Reset`)))))

(fn `UserConstructionScript`)